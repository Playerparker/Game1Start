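; Stealth enemy character that patrols, investigates noises, chases the player on sight and sends them back to a checkpoint with a melee hit.
; Tick uses boolean flags to pick chasing, target-point patrol or random wandering, each run through AIMoveTo.
; PawnSensing sets visibility, with a retriggerable delay for losing sight, and diverts the enemy to heard noises.
; Attacks use montage notifies for sparks and a hand-socket sphere trace, repeating until one lands.
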(event `self.ReceiveBeginPlay`)

(event `self.ReceiveTick`
  (params (DeltaSeconds :type "Float (single-precision)"))
  (bind _bplayervisible (`self.BPlayerVisible`))
  (if (`self.BCanMove`)
    (if _bplayervisible
      (`self.Chase Player`)
      (elif (`self.BTargetPointMove`)
        (`self.MoveToNextPoint`)
        (else
          (`self.PatrolRandom`))))
    (elif _bplayervisible
      (`self.Chase Player`))))

(event `self.PawnSensing.OnSeePawn`
  (params (Pawn :type "Pawn Object Reference"))
  (`|ExecutionSequence`
    (:`then_0`
      (cast `/Game/StealthGame/Core/Characters/PlayerCharacter/BP_ThirdPersonCharacterCustom` Pawn
        (:`then`
          (`KismetSystemLibrary.PrintString` "STOP RIGHT THERE CRIMINAL SCUM!" true true (struct :`R` 1.0 :`G` 0.02345 :`A` 1.0))
          ;[0.4911 1 0 0.5] Remember to turn on
          (set `self.BPlayerVisible` true))
        (:`CastFailed`
          (set `self.BPlayerVisible` false))))
    (:`then_1`
      (`KismetSystemLibrary.RetriggerableDelay` 2.0)
      (set `self.BPlayerVisible` false)
      (`KismetSystemLibrary.PrintString` "Keep guard, they're around here somewhere" true true (struct :`R` 0.135811 :`G` 1.0 :`A` 1.0))
      (`self.PatrolRandom`)
      (`KismetSystemLibrary.Delay` 10.0)
      (`KismetSystemLibrary.PrintString` "Slippery devil has elluded us, return to post")
      (`self.MoveToNextPoint`))))

(event `Chase Player`
  (`self.UpdateWalkSpeed` 400.0)
  (set `self.BCanMove` false)
  (`|AIMoveTo` self (0.0 0.0 0.0) (`GameplayStatics.GetPlayerCharacter` 0) 75.0
    (:`OnSuccess`
      (`self.Attack`))))

(event `PatrolRandom`
  (`KismetSystemLibrary.PrintString` "patrolling random" true true (struct :`G` 1.0 :`A` 1.0))
  (`self.UpdateWalkSpeed` 200.0)
  (set `self.BCanMove` false)
  (`|AIMoveTo` self (`NavigationSystemV1.K2_GetRandomReachablePointInRadius` (stale `self.PawnSensing.OnHearNoise` Location) 500.0 null null) null 25.0
    (:`OnSuccess`
      (`KismetSystemLibrary.Delay` 1.0)
      (set `self.BCanMove` true))))

(event `MoveToNextPoint`
  (`KismetSystemLibrary.PrintString` "HELLO I AM MOVING" true true (struct :`R` 1.0 :`G` 0.163147 :`B` 0.253581 :`A` 1.0))
  (`self.UpdateWalkSpeed` 200.0)
  (set `self.BCanMove` false)
  (`|AIMoveTo` self (0.0 0.0 0.0) (`|GetArrayItem` (`self.TargetPoints`) (`self.PatrolTargetPointIndex`)) 25.0
    (:`OnSuccess`
      (`KismetSystemLibrary.PrintString` "Made it")
      (`KismetSystemLibrary.Delay` 1.0)
      (set `self.BCanMove` true)
      (`self.SetNextPointIndex`))))

(event `SetNextPointIndex`
  (set `self.PatrolTargetPointIndex` (mod (+ (`self.PatrolTargetPointIndex`) 1) (`KismetArrayLibrary.Array_Length` (`self.TargetPoints`)))))

(event `self.PawnSensing.OnHearNoise`
  (params (Instigator :type "Pawn Object Reference") (Location :type "Vector Structure (by ref)") (Volume :type "Float (single-precision)"))
  (`KismetSystemLibrary.PrintString` "heard noise" true true (struct :`G` 1.0 :`A` 1.0))
  (`self.UpdateWalkSpeed` 200.0)
  (set `self.BCanMove` false)
  (`|AIMoveTo` self Location null 20.0
    (:`OnSuccess`
      (set `self.BCanMove` true)
      (set `self.BTargetPointMove` false)
      (`KismetSystemLibrary.Delay` (`self.RandomPatrolLength`))
      (set `self.BTargetPointMove` true)
      (`KismetSystemLibrary.PrintString` "Slippery devil has elluded us, return to post")
      (`self.MoveToNextPoint`))))

(event `Attack`
  (bind _returnvalue (`SceneComponent.GetSocketLocation` (`self.Mesh`) "hand_r"))
  ;[0.15 0.1407 0.04319 0.5] Bonk
  (`/Engine/EditorBlueprintResources/StandardMacros.DoOnce` false :!label _label ; Only Reset Attack on miss.
    (:`Completed`
      (bind _notifyname (`|PlayMontage` (`self.Mesh`) "/Game/StealthGame/Characters/Enemies/AM_Attack_01.AM_Attack_01") ; Play the AM_Attack_01
        (:`OnCompleted`
          (if (`self.bHostile`)
            (`self.ResetAttack`) ; Resets the Do Once node.
          ))
        (:`OnNotifyBegin`
          (`NiagaraFunctionLibrary.SpawnSystemAtLocation` "/Game/DevFolder/VFX/NS_Sparks.NS_Sparks" _returnvalue)
          (switch `name` _notifyname ; Pick the proper attack type(standard when there is more than one type of attack)
            (:`AttackDamage`
              (`KismetSystemLibrary.PrintString` "I'm attacking!")
              (bind (_outhits _returnvalue_2) (`KismetSystemLibrary.SphereTraceMultiForObjects` :`Start` _returnvalue :`End` (+ _returnvalue (* (`self.GetActorForwardVector`) (`self.MeleeTraceDistance`))) :`Radius` (`self.MeleeTraceRadius`) :`ObjectTypes` (`|MakeArray` "ObjectTypeQuery3" :!type "EObjectTypeQuery Enum") :`DrawDebugType` "ForDuration")) ; Trace forward from hand socket.
              (if _returnvalue_2
                (for _array_element _outhits
                  (bind _asbp_third_person_character_custom (cast `/Game/StealthGame/Core/Characters/PlayerCharacter/BP_ThirdPersonCharacterCustom` (`.HitActor` (`GameplayStatics.BreakHitResult` _array_element))))
                  (`/Game/StealthGame/Core/Characters/PlayerCharacter/BP_ThirdPersonCharacterCustom.LoadCheckpoint` _asbp_third_person_character_custom)
                  (set `self.bHostile` false) ; ...and stop attacking...
                )))))))))

(event `ResetAttack`
  ;[0.15 0.1407 0.04319 0.5] Bonk
  (goto _label :!via `Reset`))

(fn `UpdateWalkSpeed`
  (params (NewWalkSpeed :type "Float (double-precision)"))
  (set `CharacterMovementComponent.MaxWalkSpeed` NewWalkSpeed (`self.CharacterMovement`)))

(fn `UserConstructionScript`)