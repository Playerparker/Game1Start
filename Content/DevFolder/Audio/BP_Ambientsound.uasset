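; BP_Ambientsound is an ambient sound actor that starts playback when the player character class enters its sphere trigger.
; The construction script assigns the SoundCue and attenuation settings to the audio component and sizes the collision sphere from SphereRadius.
; Begin overlap casts to BP_ThirdPersonCharacterCustom and plays the sound from the start, with no end-overlap logic to stop it.
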(event `self.Collision.OnComponentBeginOverlap`
  (params (OverlappedComponent :type "PrimitiveComponent Object Reference") (OtherActor :type "Actor Object Reference") (OtherComp :type "PrimitiveComponent Object Reference") (OtherBodyIndex :type Integer) (bFromSweep :type Boolean) (SweepResult :type "HitResult Structure (by ref)"))
  (cast `/Game/StealthGame/Core/Characters/PlayerCharacter/BP_ThirdPersonCharacterCustom` OtherActor)
  (`AudioComponent.Play` (`self.AudioComponent  `) 0.0))

(fn `UserConstructionScript`
  (`AudioComponent.SetSound` (`self.AudioComponent  `) (`self.SoundCue`))
  (set `AudioComponent.AttenuationSettings` (`self.AmbientsoundAttentuation`) (`self.AudioComponent  `))
  (`SphereComponent.SetSphereRadius` (`self.Collision`) (`self.SphereRadius`) true))